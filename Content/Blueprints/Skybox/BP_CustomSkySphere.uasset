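; Custom sky sphere that sets up a dynamic sky material in the construction script from date, time of day and latitude.
; It converts the date to days since the spring equinox, then derives a sun vector from a daily circle tilted by latitude and lerped toward the rotated axis by a seasonal sine.
; The sun's negated Z samples curves for sky, horizon and sun colors and star visibility, alongside a cloud opacity setting.
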(fn `UserConstructionScript`
  (bind _dynamicskymat (`self.DynamicSkyMat`))
  (bind _dayssum (`self.DaysSum`))
  (bind (_x _y) (`KismetMathLibrary.BreakVector2D` (`self.TimeOfYear`)))
  (bind _returnvalue (* (`self.Latitude`) -1.0))
  (bind _returnvalue_2 (/ (+ (* 3600 (.x (`self.TimeOfDay`))) (* 60 (.y (`self.TimeOfDay`))) (.z (`self.TimeOfDay`))) (/ 86400.0 (`KismetMathLibrary.MultiplyByPi` 2.0))))
  (bind _z (.z (`KismetMathLibrary.VLerp` (`KismetMathLibrary.RotateAngleAxis` (`KismetMathLibrary.MakeVector` 0.0 (`KismetMathLibrary.Sin` _returnvalue_2) (`KismetMathLibrary.Cos` _returnvalue_2)) _returnvalue (0.0 1.0 0.0)) (`KismetMathLibrary.RotateAngleAxis` (1.0 0.0 0.0) _returnvalue (0.0 1.0 0.0)) (* (`KismetMathLibrary.Sin` (* (`KismetMathLibrary.Lerp` -1.0 1.0 (/ (`KismetMathLibrary.Conv_IntToDouble` (`self.DaysSum`)) 365.0)) (`KismetMathLibrary.GetPI`))) (/ 32.0 90.0)))))
  (bind _returnvalue_3 (* -1 _z))
  (bind _returnvalue_4 (`CurveLinearColor.GetLinearColorValue` (`self.SunColorCurve`) _returnvalue_3))
  (bind _returnvalue_5 (`CurveLinearColor.GetLinearColorValue` (`self.SkyBaseColorCurve`) _returnvalue_3))
  (bind _returnvalue_6 (`CurveLinearColor.GetLinearColorValue` (`self.SkyHorizonColorCurve`) _returnvalue_3))
  (bind _returnvalue_7 (`PrimitiveComponent.CreateDynamicMaterialInstance` (`self.SkySphere`) 0 null "None"))
  (set `self.DynamicSkyMat` _returnvalue_7)
  ;[1 1 1] Day of Year
  (set `self.DaysSum` 0)
  (for _index (range (+ (- (`KismetMathLibrary.FTrunc` _y) 2) 1))
    (set `self.DaysSum` (+ (`|GetArrayItem` (`self.DayPerMonth`) _index) (`self.DaysSum`))))
  (set `self.DaysSum` (+ (`self.DaysSum`) (`KismetMathLibrary.FTrunc` _x)))
  (if (> _dayssum 79)
    (set `self.DaysSum` (- _dayssum 79))
    (else
      (set `self.DaysSum` (- 365 (- 79 _dayssum)))))
  (`MaterialInstanceDynamic.SetVectorParameterValue` _dynamicskymat "SunPosition" (make `LinearColor` (.x (`KismetMathLibrary.VLerp` (`KismetMathLibrary.RotateAngleAxis` (`KismetMathLibrary.MakeVector` 0.0 (`KismetMathLibrary.Sin` _returnvalue_2) (`KismetMathLibrary.Cos` _returnvalue_2)) _returnvalue (0.0 1.0 0.0)) (`KismetMathLibrary.RotateAngleAxis` (1.0 0.0 0.0) _returnvalue (0.0 1.0 0.0)) (* (`KismetMathLibrary.Sin` (* (`KismetMathLibrary.Lerp` -1.0 1.0 (/ (`KismetMathLibrary.Conv_IntToDouble` (`self.DaysSum`)) 365.0)) (`KismetMathLibrary.GetPI`))) (/ 32.0 90.0)))) (.y (`KismetMathLibrary.VLerp` (`KismetMathLibrary.RotateAngleAxis` (`KismetMathLibrary.MakeVector` 0.0 (`KismetMathLibrary.Sin` _returnvalue_2) (`KismetMathLibrary.Cos` _returnvalue_2)) _returnvalue (0.0 1.0 0.0)) (`KismetMathLibrary.RotateAngleAxis` (1.0 0.0 0.0) _returnvalue (0.0 1.0 0.0)) (* (`KismetMathLibrary.Sin` (* (`KismetMathLibrary.Lerp` -1.0 1.0 (/ (`KismetMathLibrary.Conv_IntToDouble` (`self.DaysSum`)) 365.0)) (`KismetMathLibrary.GetPI`))) (/ 32.0 90.0)))) _z))
  (`MaterialInstanceDynamic.SetVectorParameterValue` _dynamicskymat "SkyBaseColor" _returnvalue_5)
  (set `self.SkyBaseColor` _returnvalue_5)
  (`MaterialInstanceDynamic.SetVectorParameterValue` _dynamicskymat "SkyHorizonColor" _returnvalue_6)
  (set `self.SkyHorizonColor` _returnvalue_6)
  (`MaterialInstanceDynamic.SetVectorParameterValue` _dynamicskymat "SunColor" _returnvalue_4)
  (set `self.SunColor` _returnvalue_4)
  (`MaterialInstanceDynamic.SetScalarParameterValue` _dynamicskymat "StarsVisibility" (`CurveFloat.GetFloatValue` (`self.StarsBrightnessCurve`) _returnvalue_3))
  (`MaterialInstanceDynamic.SetScalarParameterValue` _dynamicskymat "CloudsOpacity" (`self.CloudsOpacity`)))