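; PickableObject is an actor that the player can target for selection by walking into its overlap volume.
; On begin overlap with a MainCharacter it sets itself as that character's TargetToLookAt, and on end overlap it clears the target.
; Both events share one path that passes the prompt text, "E to select" or empty, to the FirstPersonView HUD for drawing.
; The selection input itself is not handled here.
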(event `self.ReceiveActorBeginOverlap`
  (params (OtherActor :type "Actor Object Reference"))
  (bind _asmain_character (cast `/Game/Blueprints/Player/MainCharacter` OtherActor))
  (set `/Game/Blueprints/Player/MainCharacter.Target to LookAt` self _asmain_character)
  (set `self.Text` "E to select")
  (bind _asfirst_person_view (cast `/Game/Blueprints/HUD/FirstPersonView` (`PlayerController.GetHUD` (`GameplayStatics.GetPlayerController` 0)) :!label _label))
  (`/Game/Blueprints/HUD/FirstPersonView.DrawTextToScreen` _asfirst_person_view true (`self.Text`)))

(event `self.ReceiveActorEndOverlap`
  (params (OtherActor :type "Actor Object Reference"))
  (bind _asmain_character (cast `/Game/Blueprints/Player/MainCharacter` OtherActor))
  (set `/Game/Blueprints/Player/MainCharacter.Target to LookAt` null _asmain_character)
  (set `self.Text` "")
  (goto _label))

(fn `UserConstructionScript`)