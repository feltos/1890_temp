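; MainCharacter is the player character Blueprint, handling basic movement and camera look through input axis events.
; Forward and strafe input move the character relative to control-rotation yaw only, ignoring pitch and roll.
; Look input drives controller yaw and pitch with per-axis sensitivity, with rate and delta-time scaling for gamepad-style handlers.
; CameraTurnMouse has two handlers, one rate-scaled and one direct, while pitch uses separate gamepad and mouse axes.
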(event `InputAxis|Forward/Backward`
  (params (AxisValue :type "Float (single-precision)"))
  ;[1 1 1] Basic Movement
  (`self.AddMovementInput` (`KismetMathLibrary.GetForwardVector` (`KismetMathLibrary.MakeRotator` 0.0 0.0 (.yaw (`self.GetControlRotation`)))) AxisValue))

(event `InputAxis|Left/Right`
  (params (AxisValue :type "Float (single-precision)"))
  ;[1 1 1] Basic Movement
  (`self.AddMovementInput` (`KismetMathLibrary.GetRightVector` (`KismetMathLibrary.MakeRotator` 0.0 0.0 (.yaw (`self.GetControlRotation`)))) AxisValue))

(event `InputAxis|CameraTurnMouse`
  (params (AxisValue :type "Float (single-precision)"))
  (`self.AddControllerYawInput` (* AxisValue (`self.CameraTurnRate`) (`self.CameraSensitivityX`) (`GameplayStatics.GetWorldDeltaSeconds`))))

(event `InputAxis|CameraLookGamePad`
  (params (AxisValue :type "Float (single-precision)"))
  (`self.AddControllerPitchInput` (* AxisValue (`self.CameraLookRate`) (`self.CameraSensitivityY`) (`GameplayStatics.GetWorldDeltaSeconds`))))

(event `InputAxis|CameraTurnMouse`
  (params (AxisValue :type "Float (single-precision)"))
  (`self.AddControllerYawInput` (* AxisValue (`self.CameraSensitivityX`))))

(event `InputAxis|CameraLookMouse`
  (params (AxisValue :type "Float (single-precision)"))
  (`self.AddControllerPitchInput` (* AxisValue (`self.CameraSensitivityY`))))

(fn `UserConstructionScript`)